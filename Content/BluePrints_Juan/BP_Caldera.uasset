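; Boiler (caldera) actor with a Pitch gauge that the player lowers by feeding it coal.
; BeginPlay starts a looping half-second timer and caches the WBP_Caldera widget from its widget component.
; Addpitch increments Pitch and writes it, clamped and normalized, to the progress bar.
; Pressing F consumes the first-person character's held item to reduce Pitch, without any proximity check or immediate bar refresh.
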(event Custom|Add%20pitch
  (bind _result (Math|Float|IncrementFloat (Variables|Default|Getpitch))
    (:%20%20
      (bind _output_get (Variables|Default|SetPorcentajeCaldera (/ (Math|Float|Clamp(Float) _result 0.0 1e+02) 1e+02)))
      (Progress|SetPercent (Variables|/Game/BluePrints_Juan/WBP_Caldera.WBP_Caldera_C|GetProgressBarCaldera (Variables|Default|GetCaldera%20Widget)) _output_get))))

(event EventBeginPlay
  (Utilities|Time|SetTimerbyEvent (EventDispatchers|CreateEvent :!event Custom|Add%20pitch) 0.5 true)
  (bind _aswbp_caldera (Utilities|Casting|CastToWBP_Caldera (UserInterface|GetWidget (Variables|Default|GetWidget))))
  (Variables|Default|SetCaldera%20Widget _aswbp_caldera))

(event Input|KeyboardEvents|F
  (params (Key :type Key%20Structure :default "None"))
  (:Pressed
    (bind _asbp_first_person_character (Utilities|Casting|CastToBP_FirstPersonCharacter (Game|GetPlayerCharacter 0)))
    (if (Variables|/Game/FirstPerson/Blueprints/BP_FirstPersonCharacter.BP_FirstPersonCharacter_C|GetHaveItem _asbp_first_person_character)
      (Development|PrintString "si hay carbon")
      (Variables|Default|Setpitch (- (Variables|Default|Getpitch) 1e+01))
      (Variables|/Game/FirstPerson/Blueprints/BP_FirstPersonCharacter.BP_FirstPersonCharacter_C|SetHaveItem _asbp_first_person_character false)
      (else
        (Development|PrintString "no hay carbon")))))

(fn ConstructionScript)

(fn UpdatePitchBar)