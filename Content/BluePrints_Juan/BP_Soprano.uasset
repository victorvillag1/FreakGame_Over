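; BP_Soprano is a singing enemy that fires a BP_OndaSoprano wave at the player on a looping timer.
; On BeginPlay it caches its anim blueprint and starts the singing audio and attack timer.
; Tick steps audio volume down as boiler percentage rises, muting near full, and deepens foldback distortion as pressure climbs.
; Muting also calls DisableInput but leaves the timer running; a player stun chain is left unwired.
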(event Custom|AtacarJugador
  (bind _returnvalue (Transformation|GetActorLocation))
  (Game|SpawnActorfromClass "/Game/FirstPerson/Blueprints/GameFunction/BP_OndaSoprano.BP_OndaSoprano_C" (Math|Transform|MakeTransform (+ _returnvalue "0.000000,0.000000,150.000000") (Math|Rotator|FindLookatRotation _returnvalue (Transformation|GetActorLocation (Game|GetPlayerCharacter 0)))) "Undefined" "MultiplyWithRoot" 0 0))

(event EventTick
  (params (DeltaSeconds :type Float%20%28single-precision%29))
  (bind _calderaref (Variables|Default|GetCalderaRef))
  (bind _presionref (Variables|Default|GetPresionRef))
  (bind _porcentajecaldera (Variables|/Game/BluePrints_Juan/BP_Caldera.BP_Caldera_C|GetPorcentajeCaldera _calderaref))
  (bind _porcentajepresion (Variables|/Game/BluePrints_Juan/BP_Presion.BP_Presion_C|GetPorcentajePresion _presionref))
  (Utilities|FlowControl|Sequence
    (:then_0
      (if (<= _porcentajecaldera 0.7)
        (bind _output_get (Variables|Default|SetVolumenCaldera 1.5))
        (Audio|Components|Audio|SetVolumeMultiplier (Variables|Default|GetAudio_Soprano) _output_get :!class /Script/Engine.AudioComponent)
        (elif (<= _porcentajecaldera 0.8)
          (bind _output_get_2 (Variables|Default|SetVolumenCaldera 1.0))
          (Audio|Components|Audio|SetVolumeMultiplier (Variables|Default|GetAudio_Soprano) _output_get_2 :!class /Script/Engine.AudioComponent)
          (elif (<= _porcentajecaldera 0.98)
            (bind _output_get_3 (Variables|Default|SetVolumenCaldera 0.5))
            (Audio|Components|Audio|SetVolumeMultiplier (Variables|Default|GetAudio_Soprano) _output_get_3 :!class /Script/Engine.AudioComponent)
            (elif (> _porcentajecaldera 0.99)
              (bind _output_get_4 (Variables|Default|SetVolumenCaldera 0.0))
              (Audio|Components|Audio|SetVolumeMultiplier (Variables|Default|GetAudio_Soprano) _output_get_4 :!class /Script/Engine.AudioComponent)
              (Input|DisableInput 0))))))
    (:then_1
      (if (>= _porcentajepresion 9e+01)
        (Variables|Default|SetDistorsionPresion -2e+01)
        (Class|SourceEffectFoldbackDistortionPreset|SetSettings (Variables|Default|GetDistorsionRef) (Utilities|Struct|MakeSourceEffectFoldbackDistortionSettings 0.0 (stale _output_get_5) -2.0) :!label _label)
        (elif (>= _porcentajepresion 75.0)
          (Variables|Default|SetDistorsionPresion -15.0)
          (goto _label)
          (elif (>= _porcentajepresion 6e+01)
            (Variables|Default|SetDistorsionPresion -1e+01)
            (goto _label)
            (elif (<= _porcentajepresion 59.9)
              (bind _output_get_5 (Variables|Default|SetDistorsionPresion 0.0))
              (goto _label))))))))

(event EventBeginPlay
  (Utilities|FlowControl|Sequence
    (:then_0
      (bind _bake_animation_attackv02_the_soprano_vip_game (Variables|Default|GetBake_Animation_AttackV02_The_Soprano_VIP_Game)
        (:then
          (bind _asabp_soprano (Utilities|Casting|CastToABP_Soprano (Components|SkeletalMesh|GetAnimInstance _bake_animation_attackv02_the_soprano_vip_game)))
          (Variables|Default|SetAnimBPRef _asabp_soprano)
          (Development|PrintString "cast succes"))
        (:else)))
    (:then_1
      (Audio|Components|Audio|Play (Variables|Default|GetAudio_Soprano) 0.0)
      (Utilities|Time|SetTimerbyEvent (delegate Custom|AtacarJugador) 8.0 true))))

(fn ConstructionScript)