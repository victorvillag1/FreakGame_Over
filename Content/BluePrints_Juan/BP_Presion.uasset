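; BP_Presion is a pressure gauge Blueprint that tracks a Pitch value and shows it on a WBP_Presion progress bar in a widget component.
; BeginPlay starts a looping timer and caches the widget.
; Addpitch increments Pitch and updates the bar as a fraction of 100, while pressing E lowers Pitch.
; The clamp feeds only PorcentajePresion and its debug print, so Pitch itself stays unbounded.
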(event Custom|Add%20pitch
  (bind _result (Math|Float|IncrementFloat (Variables|Default|Getpitch))
    (:%20%20
      (bind _output_get (Variables|Default|SetPorcentajePresion (Math|Float|Clamp(Float) _result 0.0 1e+02)))
      (Development|PrintString (Utilities|String|ToString(Float) _output_get))
      (Progress|SetPercent (Variables|/Game/BluePrints_Juan/WBP_Presion.WBP_Presion_C|GetProgressBarPresion (Variables|Default|GetPression%20Widget)) (/ (Variables|Default|Getpitch) 1e+02)))))

(event EventBeginPlay
  (Utilities|Time|SetTimerbyEvent (EventDispatchers|CreateEvent :!event Custom|Add%20pitch) 0.5 true)
  (bind _aswbp_presion (Utilities|Casting|CastToWBP_Presion (UserInterface|GetWidget (Variables|Default|GetWidget))))
  (Variables|Default|SetPression%20Widget _aswbp_presion))

(event Input|KeyboardEvents|E
  (params (Key :type Key%20Structure :default "None"))
  (:Pressed
    (Variables|Default|Setpitch (- (Variables|Default|Getpitch) 3.0))))

(fn ConstructionScript)